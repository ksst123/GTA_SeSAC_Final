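; BP_GTAPlayer02 is a player Blueprint with a GTA-style pie menu for equipping weapons, plus a health bar created at BeginPlay.
; Holding the Tap input shows a new GTAPieMenu in Game and UI mode; releasing it ends selection and restores game-only input.
; Left-clicking while it is open reads the selection to set a left or right arm mesh, or clear both and destroy WeaponRef.
; The fourth option does nothing.
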(event Collision|EventActorBeginOverlap
  (params (OtherActor :type Actor%20Object%20Reference)))

(event EventTick
  (params (DeltaSeconds :type Float%20%28single-precision%29)))

(event EventBeginPlay
  (bind _returnvalue (UserInterface|CreateWidget "/Game/Seung/UI/HealthBar/HealthBar.HealthBar_C"))
  (UserInterface|Viewport|AddtoViewport _returnvalue 0))

(event Input|ActionEvents|InputActionTap
  (params (Key :type Key%20Structure))
  (bind _returnvalue (Game|GetPlayerController 0))
  (bind _returnvalue_2 (Game|GetPlayerController 0))
  (:Pressed
    (Variables|Default|SetWindowisOpen? true)
    (bind _returnvalue_3 (UserInterface|CreateWidget "/Game/Seung/UI/PieMenu/GTAPieMenu.GTAPieMenu_C"))
    (Default|StartSelection _returnvalue_3)
    (bind _output_get (Variables|Default|SetPieMenuRef _returnvalue_3))
    (UserInterface|Viewport|AddtoViewport _output_get 0)
    (Variables|/Script/Engine.PlayerController|SetbShowMouseCursor _returnvalue_2 false)
    (Input|SetIgnoreLookInput _returnvalue_2 false)
    (Input|SetInputModeGameandUI _returnvalue_2 _output_get "DoNotLock" true false))
  (:Released
    (Variables|Default|SetWindowisOpen? false)
    (Default|EndSelction (Variables|Default|GetPieMenuRef))
    (Widget|RemovefromParent (Variables|Default|GetPieMenuRef))
    (Variables|/Script/Engine.PlayerController|SetbShowMouseCursor _returnvalue false)
    (Input|SetIgnoreLookInput _returnvalue false)
    (Input|SetInputModeGameOnly _returnvalue false)))

(event Input|MouseEvents|LeftMouseButton
  (params (Key :type Key%20Structure))
  (:Pressed
    (if (Variables|Default|GetWindowisOpen?)
      (bind (_i1 _i2 _i3 _i4) (Default|CallSelection (Variables|Default|GetPieMenuRef)))
      (if _i2
        (Components|SkeletalMesh|SetSkeletalMeshAsset (Variables|Default|GetLeftArmSlot) "/Game/Seung/Guns/Pistol04/source/textures.textures")
        (elif _i3
          (Components|SkeletalMesh|SetSkeletalMeshAsset (Variables|Default|GetRightArmSlot) "/Game/Seung/Guns/SniperGun02/Cheytac_M200_Intrevention.Cheytac_M200_Intrevention")
          (elif _i1
            (Components|SkeletalMesh|SetSkeletalMeshAsset (Variables|Default|GetLeftArmSlot) 0)
            (Components|SkeletalMesh|SetSkeletalMeshAsset (Variables|Default|GetRightArmSlot) 0)
            (Actor|DestroyActor (Variables|Default|GetWeaponRef))
            (elif _i4
              _)))))))

(fn ConstructionScript)