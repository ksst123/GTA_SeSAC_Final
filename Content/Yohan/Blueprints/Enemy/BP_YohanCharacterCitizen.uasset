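; Citizen character Blueprint with player input for sprinting and weapon selection, plus HUD hooks for ammo and mission text.
; Run input switches walk speed and starts self-recursing delayed events that drain or regenerate stamina, stopping the run at zero.
; Holding Tap shows a GTA-style pie menu, where WeaponChange selects pistol or hands.
; BeginPlay creates mission and main widgets; several stance, crosshair and stamina-widget chains are left unwired.
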(event Custom|RegenStamina
  (bind _output_get (Variables|Default|SetStamina (Math|Integer|Clamp(Integer) (+ (Variables|Default|GetStamina) 1) 0 (Variables|Default|GetMaxStamina))))
  (if (not (== _output_get (Variables|Default|GetMaxStamina)))
    (if (not (Variables|Default|GetIsRunning))
      (Utilities|FlowControl|Delay 0.05)
      (CallFunction|RegenStamina))))

(event Custom|DrainStamina
  (bind _output_get (Variables|Default|SetStamina (Math|Integer|Clamp(Integer) (- (Variables|Default|GetStamina) 2) 0 (Variables|Default|GetMaxStamina))))
  (if (== _output_get 0)
    (CallFunction|StopRun)
    (elif (Variables|Default|GetIsRunning)
      (Utilities|FlowControl|Delay 0.1)
      (CallFunction|DrainStamina))))

(event Input|EnhancedActionEvents|EnhancedInputActionIA_Run
  (params (ActionValue :type Boolean) (ElapsedSeconds :type Float%20%28double-precision%29) (TriggeredSeconds :type Float%20%28double-precision%29) (InputAction :type Input%20Action%20Object%20Reference :default "/Game/Yohan/Input/Actions/IA_Run.IA_Run"))
  (:Triggered
    (CallFunction|StartRun))
  (:Completed
    (CallFunction|StopRun)))

(event EventBeginPlay
  (bind _returnvalue (UserInterface|CreateWidget "/Game/Yohan/UI/WB_Mission.WB_Mission_C" (Game|GetPlayerController 0)))
  (Variables|Default|SetMissionWidget _returnvalue)
  (Utilities|FlowControl|Sequence
    (:then_0
      (if (== (Game|GetPlayerController 0) (Pawn|GetController self))
        (bind _returnvalue_2 (UserInterface|CreateWidget "/Game/Yohan/UI/WB_Main.WB_Main_C"))
        (bind _output_get (Variables|Default|SetMainUI _returnvalue_2))
        (UserInterface|Viewport|AddtoViewport _output_get 0)))))

(event Collision|EventActorBeginOverlap
  (params (OtherActor :type Actor%20Object%20Reference)))

(event EventTick
  (params (DeltaSeconds :type Float%20%28single-precision%29)))

(event EventOnMyPistolAmmoUpdate
  (params (current :type Integer) (max :type Integer))
  (Default|UpdatePistolAmmo (Variables|/Game/Yohan/UI/WB_Main.WB_Main_C|GetWB_Weapon (Variables|Default|GetMainUI)) current max))

(event Input|ActionEvents|InputActionTap
  (params (Key :type Key%20Structure :default "None"))
  (bind _returnvalue (Game|GetPlayerController 0))
  (bind _returnvalue_2 (Game|GetPlayerController 0))
  ;[1 1 1] PieMenu
  (:Pressed
    (Variables|Default|SetWindowisOpen? true)
    (bind _returnvalue_3 (UserInterface|CreateWidget "/Game/Seung/UI/PieMenu/GTAPieMenu.GTAPieMenu_C"))
    (Default|StartSelection _returnvalue_3)
    (bind _output_get (Variables|Default|SetPieMenuRef _returnvalue_3))
    (UserInterface|Viewport|AddtoViewport _output_get 0)
    (Variables|/Script/Engine.PlayerController|SetbShowMouseCursor _returnvalue_2 false)
    (Input|SetIgnoreLookInput _returnvalue_2 false)
    (Input|SetInputModeGameandUI _returnvalue_2 _output_get "DoNotLock" true false))
  (:Released
    (Variables|Default|SetWindowisOpen? false)
    (Default|EndSelction (Variables|Default|GetPieMenuRef))
    (Widget|RemovefromParent (Variables|Default|GetPieMenuRef))
    (Variables|/Script/Engine.PlayerController|SetbShowMouseCursor _returnvalue false)
    (Input|SetIgnoreLookInput _returnvalue false)
    (Input|SetInputModeGameOnly _returnvalue false)))

(event Input|ActionEvents|InputActionWeaponChange
  (params (Key :type Key%20Structure :default "None"))
  ;[1 1 1] WeaponChange
  (:Pressed
    (if (Variables|Default|GetWindowisOpen?)
      (bind (_i1 _i2 _i3 _i4) (Default|CallSelection (Variables|Default|GetPieMenuRef)))
      (if _i2
        (Class|YohanCharacter|OnActionPistol)
        (elif (not _i3)
          (if _i1
            (Class|YohanCharacter|OnActionHand)
            (elif _i4
              _)))))))

(fn ConstructionScript)

(fn StopRun
  (Variables|/Script/Engine.CharacterMovementComponent|SetMaxWalkSpeed (Variables|Character|GetCharacterMovement) 3e+02)
  (Variables|Default|SetIsRunning false)
  (CallFunction|RegenStamina))

(fn StartRun
  (Variables|/Script/Engine.CharacterMovementComponent|SetMaxWalkSpeed (Variables|Character|GetCharacterMovement) 6e+02)
  (Variables|Default|SetIsRunning true)
  (CallFunction|DrainStamina))

(fn UpdateMission
  (params (CurrentMission :type String))
  (bind _output_get (Variables|Default|SetCurrentMission CurrentMission))
  (Rendering|Components|TextRender|SetText (Variables|/Game/Yohan/UI/WB_Mission.WB_Mission_C|GetCurrentMissionText (Variables|Default|GetMissionWidget)) (Utilities|Text|ToText(String) _output_get)))