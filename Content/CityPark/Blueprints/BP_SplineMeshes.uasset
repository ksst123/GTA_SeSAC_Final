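; Construction-script Blueprint that lays a chosen static mesh along a spline as deformed spline mesh segments, each with two material overrides.
; SplineMeshVar selects the layout: one segment per pair of spline points using their tangents, or segments at fixed Spacing along the spline length.
; In spacing mode, tangents are the spline direction scaled by Spacing plus an adjustable offset.
; Both modes share the Wire graph's component creation step.
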(fn ConstructionScript
  (|Wire))